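; BP_Tile_Parent is the base Blueprint for level-generation tiles, each carrying six lanes and a trigger box.
; When a player overlaps the box, any tile except number zero reports its TileNumber to the LevelManager.
; The construction script gathers the lane components into an array and a struct.
; Cleanup functions destroy the lane splines and any NPC actors overlapping the box.
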(event `self.Box.OnComponentBeginOverlap`
  (params (OverlappedComponent :type "PrimitiveComponent Object Reference") (OtherActor :type "Actor Object Reference") (OtherComp :type "PrimitiveComponent Object Reference") (OtherBodyIndex :type Integer) (bFromSweep :type Boolean) (SweepResult :type "HitResult Structure (by ref)"))
  (if (not (== (`self.TileNumber`) 0))
    (cast `/Game/Player/BP_Player_Parent` OtherActor)
    (`/Game/LevelGeneration/BP_RandomWorldGenerator.EventPlayerEntersNewTile` (`self.LevelManager`) (`self.TileNumber`))))

(fn `DestroySplines`
  (for _array_element (`self.LaneArray`)
    (`ActorComponent.K2_DestroyComponent` _array_element)))

(fn `DestroyVehicles`
  (for _array_element (`PrimitiveComponent.GetOverlappingActors` (`self.Box`) "/Game/NPC/BP_NPC_Parent.BP_NPC_Parent_C")
    (`self.K2_DestroyActor` _array_element))
  (return))

(fn `UserConstructionScript`
  (bind _lane01 (`self.Lane01`))
  (bind _lane02 (`self.Lane02`))
  (bind _lane03 (`self.Lane03`))
  (bind _lane06 (`self.Lane06`))
  (bind _lane05 (`self.Lane05`))
  (bind _lane04 (`self.Lane04`))
  (set `self.LaneArray` (`|MakeArray` _lane01 _lane02 _lane03 _lane04 _lane05 _lane06))
  (set `self.LaneStruct` (make `/Game/LevelGeneration/Tiles/STUCT_Lane` _lane01 _lane02 _lane03 _lane04 _lane05 _lane06)))