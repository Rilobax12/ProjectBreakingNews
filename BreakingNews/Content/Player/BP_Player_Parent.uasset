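; Parent Blueprint for the player's car in a car-chase game, passing throttle, steering and handbrake input to the vehicle.
; Steering input scales down as speed rises and, with no input, self-straightens toward the world X axis.
; Tick only prints a debug mph readout.
; Lane-spline look-ahead steering, lane switching, impact-based crash detection and distance scoring to a news ticker remain in the graph but are disconnected, so never run.
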(event `InputAxis|Steering`
  (params (AxisValue :type "Float (single-precision)"))
  (bind _returnvalue (/ 1000.0 (`KismetMathLibrary.VSize` (`self.GetVelocity`))))
  (`KismetSystemLibrary.PrintString` (`KismetStringLibrary.Conv_DoubleToString` _returnvalue) true true (struct :`G` 0.66 :`B` 1.0 :`A` 1.0) (`GameplayStatics.GetWorldDeltaSeconds`))
  (`self.SetSteering` (`KismetMathLibrary.SelectFloat` (* AxisValue (`KismetMathLibrary.FClamp` _returnvalue 0.1)) (* (`KismetMathLibrary.Dot_VectorVector` (`self.GetActorForwardVector`) (0.0 -1.0 0.0)) 1.0) (> (`KismetMathLibrary.Abs` AxisValue) 0.0))))

(event `self.ReceiveBeginPlay`
  (`self.InitializeAllSystems`)
  (`PlayerController.ClientStartCameraShake` :`self` (`GameplayStatics.GetPlayerController` 0) :`Shake` "/Game/Player/CS_Chase.CS_Chase_C" :`Scale` 0.0))

(event `InputAxis|Throttle`
  (params (AxisValue :type "Float (single-precision)"))
  (`self.SetEngineThrottle` (`KismetMathLibrary.FClamp` AxisValue -1.0)))

(event `Steering`
  (params (DeltaSeconds :type "Float (double-precision)"))
  (bind _returnvalue (`self.K2_GetActorLocation`))
  (bind _returnvalue_2 (`self.K2_GetActorLocation`))
  (bind _lanespline_ref (`self.LaneSpline_Ref`))
  (bind _returnvalue_3 (`SplineComponent.FindLocationClosestToWorldLocation` (`self.LaneSpline_Ref`) (+ _returnvalue (* (`SplineComponent.FindDirectionClosestToWorldLocation` _lanespline_ref (`self.K2_GetActorLocation`) "World") (* (+ (/ (`KismetMathLibrary.VSize` (`KismetMathLibrary.ProjectVectorOnToVector` (`self.GetVelocity`) (1.0 0.0 0.0))) 2.0) (`KismetMathLibrary.VSize` (- (`SplineComponent.FindLocationClosestToWorldLocation` _lanespline_ref _returnvalue_2 "World") _returnvalue_2))) (`KismetMathLibrary.SelectFloat` 1.0 -1.0 (<= (`self.Lane`) 2))))) "World"))
  (set `self.Target` _returnvalue_3)
  (`self.SetSteering` (`KismetMathLibrary.Dot_VectorVector` (`KismetMathLibrary.Conv_RotatorToVector` (`KismetMathLibrary.FindLookAtRotation` _returnvalue _returnvalue_3)) (`self.GetActorRightVector`))))

(event `InputAction|Handbrake`
  (params (Key :type "Key Structure"))
  (:`Pressed`
    (`self.SetHandbrake` true))
  (:`Released`
    (`self.SetHandbrake` false)))

(event `self.StaticMesh.OnComponentHit`
  (params (HitComponent :type "PrimitiveComponent Object Reference") (OtherActor :type "Actor Object Reference") (OtherComp :type "PrimitiveComponent Object Reference") (NormalImpulse :type "Vector Structure") (Hit :type "HitResult Structure (by ref)")))

(event `self.ReceiveTick`
  (params (DeltaSeconds :type "Float (single-precision)"))
  (`KismetSystemLibrary.PrintString` (`KismetStringLibrary.Concat_StrStr` (`KismetTextLibrary.Conv_TextToString` (`KismetTextLibrary.Conv_DoubleToText` (* (`KismetMathLibrary.VSize` (`self.GetVelocity`)) 0.022369) "HalfToEven" false true 2 324 0 0)) " mph") true true (struct :`G` 0.66 :`B` 1.0 :`A` 1.0) DeltaSeconds))

(fn `UserConstructionScript`)